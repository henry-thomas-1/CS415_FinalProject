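; Weeping Angel enemy that, once alerted by sight, pursues the player's last seen location but halts while the camera faces it.
; Tick runs a camera dot-product check, using self-targeted AIMoveTo to stop and turn toward the player.
; Heard noises stop it and, before alert, rotate it toward the sound.
; Self-repeating events handle HitBox damage, zeroed at BeginPlay, and surface-based footsteps, traced beneath the player pawn rather than itself.
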(event OnComponentBeginOverlap(HitBox)
  (params (OverlappedComponent :type Primitive%20Component%20Object%20Reference) (OtherActor :type Actor%20Object%20Reference) (OtherComp :type Primitive%20Component%20Object%20Reference) (OtherBodyIndex :type Integer) (bFromSweep :type Boolean) (SweepResult :type Hit%20Result%20Structure%20%28by%20ref%29))
  ;[1 1 1] Overlap Settings
  (if (== OtherActor (Game|Player|GetPlayerPawn 0))
    (Variables|Default|SetDamaging true)
    (CallFunction|BurnMF)))

(event OnComponentEndOverlap(HitBox)
  (params (OverlappedComponent :type Primitive%20Component%20Object%20Reference) (OtherActor :type Actor%20Object%20Reference) (OtherComp :type Primitive%20Component%20Object%20Reference) (OtherBodyIndex :type Integer))
  ;[1 1 1] Overlap Settings
  (if (== OtherActor (Game|Player|GetPlayerPawn 0))
    (Variables|Default|SetDamaging false)))

(event OnSeePawn(PawnSensing)
  (params (Pawn :type Pawn%20Object%20Reference))
  (Variables|Default|SetLast%20Seen%20Location (Transformation|GetActorLocation (Game|Player|GetPlayerPawn 0)))
  (Variables|Default|SetAlert true))

(event OnHearNoise(PawnSensing)
  (params (Instigator :type Pawn%20Object%20Reference) (Location :type Vector%20%28by%20ref%29 :default "0, 0, 0") (Volume :type Float%20%28single-precision%29))
  (bind _self self)
  (AI|AIMoveTo _self "0, 0, 0" _self 5.0 false
    (:then
      (CallFunction|TurnTowardsNoise Location))))

(event Custom|Turn%20Towards%20Noise
  (params (Location :type Vector))
  (bind _returnvalue (Utilities|Time|GetWorldDeltaSeconds))
  (bind _returnvalue_2 (Transformation|GetActorLocation))
  (bind _returnvalue_3 (Transformation|GetActorRotation))
  (bind _returnvalue_4 (Math|Rotator|FindLookatRotation _returnvalue_2 Location))
  (bind _returnvalue_5 (Math|Interpolation|RInterpTo _returnvalue_3 _returnvalue_4 _returnvalue 5.0))
  (if (not (Variables|Default|GetAlert))
    (Transformation|SetActorRotation (Math|Rotator|MakeRotator 0.0 0.0 (.yaw _returnvalue_5)))
    (Utilities|FlowControl|Delay 0.001)
    (if (>= (Math|Float|Absolute(Float) (- (.yaw _returnvalue_5) (.Yaw (Math|Rotator|BreakRotator _returnvalue_3)))) 0.001)
      (CallFunction|TurnTowardsNoise Location))))

(event Custom|BurnMF
  ;[1 1 1] Overlap Settings
  (if (Variables|Default|GetDamaging)
    (bind _asmaster (CallFunction|GetPlayer))
    (Default|GetDamage :self _asmaster :DamagePoint (Variables|Default|GetDamage%20Value))
    (Utilities|FlowControl|Delay (Variables|Default|GetGet%20Damage%20Each%20%28N%29%20Second%28s%29))
    (CallFunction|BurnMF)))

(event Custom|thing
  (if (Variables|Default|Getmoving)
    (CallFunction|Footstep)
    (Utilities|FlowControl|Delay (Math|Float|Min(Float) 0.5 (/ 1.5e+02 (Math|Vector|VectorLength (Transformation|GetVelocity)))))
    (CallFunction|Thing)))

(event EventBeginPlay
  (Variables|Default|SetDamage%20Value 0.0))

(event Collision|EventActorBeginOverlap
  (params (OtherActor :type Actor%20Object%20Reference)))

(event EventTick
  (params (DeltaSeconds :type Float%20%28single-precision%29))
  (bind _self self)
  (bind _charactermovement (Variables|Character|GetCharacterMovement))
  (CallFunction|Bruh)
  (if (Variables|Default|GetAlert)
    (Variables|/Script/Engine.CharacterMovementComponent|SetMaxWalkSpeed _charactermovement 6e+02)
    (bind _is_looking (CallFunction|IsLookingTowards))
    (if _is_looking
      (AI|AIMoveTo _self "0, 0, 0" _self 5.0 false
        (:then
          (CallFunction|LookatPlayer)))
      (else
        (AI|AIMoveTo self (Variables|Default|GetLast%20Seen%20Location) 0 5.0 false
          (:OnSuccess
            (Utilities|FlowControl|Delay 3.0)))))
    (else
      (Variables|/Script/Engine.CharacterMovementComponent|SetMaxWalkSpeed _charactermovement 2e+02))))

(fn ConstructionScript)

(fn IsLookingTowards
  (bind _returnvalue (Game|GetPlayerCameraManager 0))
  (bind _returnvalue_2 (Transformation|GetActorLocation))
  (bind _returnvalue_3 (Transformation|GetActorLocation _returnvalue))
  (bind _returnvalue_4 (- _returnvalue_2 _returnvalue_3))
  (return (>= (/ (Math|Vector|DotProduct (Transformation|GetActorForwardVector _returnvalue) _returnvalue_4) (Math|Vector|VectorLength _returnvalue_4)) 0.6)))

(fn LookatPlayer
  (Transformation|SetActorRotation (Math|Rotator|MakeRotator 0.0 0.0 (.yaw (Math|Interpolation|RInterpTo (Transformation|GetActorRotation) (Math|Rotator|FindLookatRotation (Transformation|GetActorLocation) (Transformation|GetActorLocation (Game|GetPlayerCharacter 0))) (Utilities|Time|GetWorldDeltaSeconds) 5.0))))
  (return))

(fn Footstep
  (bind _returnvalue (Game|Player|GetPlayerPawn 0))
  (bind _footstepsoundsettings (CallFunction|FootstepSoundSettings))
  (bind _returnvalue_2 (Pawn|GetMovementComponent))
  (bind (_default _carpet _dirt _grass _metal _rock _tile _wood) (Utilities|Struct|BreakHorrorEngine_Footstep _footstepsoundsettings))
  (bind _returnvalue_3 (Transformation|GetActorLocation _returnvalue))
  (if (Math|Boolean|ANDBoolean (> (Math|Vector|VectorLength (- (Transformation|GetActorLocation) (LocalVariables|GetCurrent%20Foot%20Location))) (Utilities|Struct|BreakHorrorEngine_Footstep (CallFunction|FootstepSoundSettings))) (AI|Components|NavMovement|IsMovingonGround _returnvalue_2) (!= (Math|Vector|VectorLength (Variables|/Script/Engine.MovementComponent|GetVelocity _returnvalue_2)) 0.0))
    (bind _outactors (Actor|GetAllActorswithTag "IgnoreTrace"))
    (bind (_outhit _returnvalue_4) (Collision|SphereTraceByChannel _returnvalue_3 (- _returnvalue_3 (Math|Vector|MakeVector 0.0 0.0 (* (Variables|/Script/Engine.CapsuleComponent|GetCapsuleHalfHeight (Variables|Collision|GetCapsuleComponent)) 2.0))) 0.0 "TraceTypeQuery1" true _outactors "None"))
    (if _returnvalue_4
      (Audio|SpawnSoundatLocation (Utilities|Select :Index (Variables|/Script/PhysicsCore.PhysicalMaterial|GetSurfaceType (.physmat _outhit)) :SurfaceType_Default _default :SurfaceType1 _carpet :SurfaceType2 _dirt :SurfaceType3 _grass :SurfaceType4 _metal :SurfaceType5 _rock :SurfaceType6 _tile :SurfaceType7 _wood) (.location _outhit) "0, 0, 0" 1.0 1.0 0.0 0 0)
      (LocalVariables|SetCurrent%20Foot%20Location (Transformation|GetActorLocation (Game|Player|GetPlayerPawn 0))))))

(fn Bruh
  (bind _returnvalue (Transformation|GetVelocity))
  (bind _returnvalue_2 (Math|Vector|VectorLength _returnvalue))
  (bind _returnvalue_3 (> _returnvalue_2 1.5e+02))
  (if (Variables|Default|Getmoving)
    (if (not _returnvalue_3)
      (Variables|Default|Setmoving false))
    (elif _returnvalue_3
      (Variables|Default|Setmoving true)
      (CallFunction|Thing))))