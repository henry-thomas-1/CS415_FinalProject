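; Car actor with three repair points, one each for replacing the tire, fixing the bumper and filling the gas.
; When the HorrorEngineCharacter enters a point's trigger, it creates and shows that task's widget unless the matching fixed or filled flag is set.
; Leaving the trigger removes the stored widget from the screen.
; The event graph only reads the completion flags and never sets them.
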(event OnComponentBeginOverlap(Tire_fix)
  (params (OverlappedComponent :type Primitive%20Component%20Object%20Reference) (OtherActor :type Actor%20Object%20Reference) (OtherComp :type Primitive%20Component%20Object%20Reference) (OtherBodyIndex :type Integer) (bFromSweep :type Boolean) (SweepResult :type Hit%20Result%20Structure%20%28by%20ref%29))
  (Utilities|Casting|CastToHorrorEngineCharacter OtherActor)
  (if (not (Variables|Default|Gettire_fixed))
    (bind _returnvalue (UserInterface|CreateWidget "/Game/Stranded_content/widgets/Replace_tire.Replace_tire_C"))
    (bind _output_get (Variables|Default|Settire_widget _returnvalue))
    (UserInterface|Viewport|AddtoViewport _output_get 0)))

(event OnComponentEndOverlap(Tire_fix)
  (params (OverlappedComponent :type Primitive%20Component%20Object%20Reference) (OtherActor :type Actor%20Object%20Reference) (OtherComp :type Primitive%20Component%20Object%20Reference) (OtherBodyIndex :type Integer))
  (Utilities|Casting|CastToHorrorEngineCharacter OtherActor)
  (Widget|RemovefromParent (Variables|Default|Gettire_widget)))

(event OnComponentBeginOverlap(Bumper_fix)
  (params (OverlappedComponent :type Primitive%20Component%20Object%20Reference) (OtherActor :type Actor%20Object%20Reference) (OtherComp :type Primitive%20Component%20Object%20Reference) (OtherBodyIndex :type Integer) (bFromSweep :type Boolean) (SweepResult :type Hit%20Result%20Structure%20%28by%20ref%29))
  (Utilities|Casting|CastToHorrorEngineCharacter OtherActor)
  (if (not (Variables|Default|Getbumper_fixed))
    (bind _returnvalue (UserInterface|CreateWidget "/Game/Stranded_content/widgets/Fix_bumper.Fix_bumper_C"))
    (bind _output_get (Variables|Default|Setbumper_widget _returnvalue))
    (UserInterface|Viewport|AddtoViewport _output_get 0)))

(event OnComponentEndOverlap(Bumper_fix)
  (params (OverlappedComponent :type Primitive%20Component%20Object%20Reference) (OtherActor :type Actor%20Object%20Reference) (OtherComp :type Primitive%20Component%20Object%20Reference) (OtherBodyIndex :type Integer))
  (Utilities|Casting|CastToHorrorEngineCharacter OtherActor)
  (Widget|RemovefromParent (Variables|Default|Getbumper_widget)))

(event OnComponentBeginOverlap(fillgas)
  (params (OverlappedComponent :type Primitive%20Component%20Object%20Reference) (OtherActor :type Actor%20Object%20Reference) (OtherComp :type Primitive%20Component%20Object%20Reference) (OtherBodyIndex :type Integer) (bFromSweep :type Boolean) (SweepResult :type Hit%20Result%20Structure%20%28by%20ref%29))
  (Utilities|Casting|CastToHorrorEngineCharacter OtherActor)
  (if (not (Variables|Default|Getgas_filled))
    (bind _returnvalue (UserInterface|CreateWidget "/Game/Stranded_content/widgets/Fill_Gas.Fill_Gas_C"))
    (bind _output_get (Variables|Default|Setgas_widget _returnvalue))
    (UserInterface|Viewport|AddtoViewport _output_get 0)))

(event OnComponentEndOverlap(fillgas)
  (params (OverlappedComponent :type Primitive%20Component%20Object%20Reference) (OtherActor :type Actor%20Object%20Reference) (OtherComp :type Primitive%20Component%20Object%20Reference) (OtherBodyIndex :type Integer))
  (Utilities|Casting|CastToHorrorEngineCharacter OtherActor)
  (Widget|RemovefromParent (Variables|Default|Getgas_widget)))

(event EventBeginPlay)

(event EventTick
  (params (DeltaSeconds :type Float%20%28single-precision%29)))

(fn ConstructionScript)