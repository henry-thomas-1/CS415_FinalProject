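; BP_Zombie is a stalker zombie AI that chases the player after pawn sensing spots them, recording their last known location.
; A camera dot-product test and a visibility trace from the player gate the chase.
; When both are true, it moves toward the player and rechecks after a delay; otherwise it targets its current position, then later the recorded location.
; ActivateRoar only sets a flag.
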(event OnSeePawn(PawnSensing)
  (params (Pawn :type Pawn%20Object%20Reference))
  (CallFunction|ChasePlayer)
  (Variables|Default|SetLast%20Known%20Location (Transformation|GetActorLocation (Game|GetPlayerCharacter 0))))

(event Custom|Chase%20Player
  (bind _self self)
  (bind _looking (CallFunction|IsLooking))
  (bind _obstructed (CallFunction|IsViewObstructed))
  (if (and _obstructed _looking)
    (AI|AIMoveTo self "0, 0, 0" (Game|GetPlayerCharacter 0) 5.0 false
      (:then
        (Utilities|FlowControl|Delay 0.5)
        (CallFunction|ChasePlayer)))
    (else
      (AI|AIMoveTo _self (Transformation|GetActorLocation _self) 0 5.0 false
        (:then
          (Utilities|FlowControl|Delay 5.0)
          (AI|AIMoveTo self (Variables|Default|GetLast%20Known%20Location) 0 5.0 false))))))

(event EventBeginPlay)

(event Collision|EventActorBeginOverlap
  (params (OtherActor :type Actor%20Object%20Reference)))

(event EventTick
  (params (DeltaSeconds :type Float%20%28single-precision%29))
  (if (Variables|Default|GetLooking%20Timer%20On)
    _))

(fn ConstructionScript)

(fn IsLooking
  (bind _returnvalue (Game|GetPlayerCameraManager 0))
  (bind _self self)
  (bind _returnvalue_2 (Transformation|GetActorLocation _self))
  (bind _returnvalue_3 (Transformation|GetActorLocation _returnvalue))
  (bind _returnvalue_4 (- _returnvalue_2 _returnvalue_3))
  (return (> (/ (Math|Vector|DotProduct (Transformation|GetActorForwardVector _returnvalue) _returnvalue_4) (Math|Vector|VectorLength _returnvalue_4)) 0.75)))

(fn IsViewObstructed
  (bind _returnvalue (Game|Player|GetPlayerPawn 0))
  (bind _returnvalue_2 (Collision|LineTraceByChannel (Transformation|GetActorLocation _returnvalue) (Transformation|GetActorLocation self) "TraceTypeQuery1" false (Utilities|Array|MakeArray _returnvalue) "None"))
  (return _returnvalue_2))

(fn ActivateRoar
  (Variables|Default|SetRoaring true))